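; Rotating platform actor that, as test behavior, endlessly flips its mesh down and back after a short delay on BeginPlay.
; Flip events use MoveComponentTo to rotate PlatformMesh over FlipTime to a direction's rotation or back to StartRotation.
; The construction script sets those rotations through Selects fixed at index 0 and resets the mesh to StartRotation.
; FlipUp, FlipLeft and FlipRight are defined but not called here.
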(event `self.ReceiveBeginPlay`
  ;[1 1 1] Test Rotation of Platform
  (`KismetSystemLibrary.Delay` 1.0)
  (`self.FlipDown` :!label _label)
  (`KismetSystemLibrary.Delay` 4.2)
  (`self.ReturnFlip`)
  (`KismetSystemLibrary.Delay` 4.2)
  (goto _label))

(event `self.ReceiveTick`
  (params (DeltaSeconds :type "Float (single-precision)"))
  ;[1 1 1] Test Rotation of Platform
)

(event `FlipUp`
  ;[1 1 1] Flip Functions
  (`KismetSystemLibrary.MoveComponentTo` (`self.PlatformMesh`) (0.0 0.0 0.0) (`self.Up`) false false (`self.FlipTime`)))

(event `FlipDown`
  ;[1 1 1] Flip Functions
  (`KismetSystemLibrary.MoveComponentTo` (`self.PlatformMesh`) (0.0 0.0 0.0) (`self.Down`) false false (`self.FlipTime`)))

(event `FlipLeft`
  ;[1 1 1] Flip Functions
  (`KismetSystemLibrary.MoveComponentTo` (`self.PlatformMesh`) (0.0 0.0 0.0) (`self.Left`) false false (`self.FlipTime`)))

(event `FlipRight`
  ;[1 1 1] Flip Functions
  (`KismetSystemLibrary.MoveComponentTo` (`self.PlatformMesh`) (0.0 0.0 0.0) (`self.Right`) false false (`self.FlipTime`)))

(event `ReturnFlip`
  ;[1 1 1] Flip Functions
  (`KismetSystemLibrary.MoveComponentTo` (`self.PlatformMesh`) (0.0 0.0 0.0) (`self.StartRotation`) false false (`self.FlipTime`)))

(fn `UserConstructionScript`
  (set `self.StartRotation` (select `int` 0 :`0` (struct) :`1` (struct) :!type "Rotator Structure"))
  (`|ExecutionSequence`
    (:`then_0`
      (set `self.Down` (select `int` 0 :`0` (struct :`Roll` -90.0) :`1` (struct) :!type "Rotator Structure"))
      (`SceneComponent.K2_SetRelativeRotation` (`self.PlatformMesh`) (`self.StartRotation`) false false))
    (:`then_1`
      (set `self.Up` (select `int` 0 :`0` (struct :`Roll` 90.0) :`1` (struct) :!type "Rotator Structure"))
      (`SceneComponent.K2_SetRelativeRotation` (`self.PlatformMesh`) (`self.StartRotation`) false false))
    (:`then_2`
      (set `self.Left` (select `int` 0 :`0` (struct :`Pitch` 20.0) :`1` (struct) :!type "Rotator Structure"))
      (`SceneComponent.K2_SetRelativeRotation` (`self.PlatformMesh`) (`self.StartRotation`) false false))
    (:`then_3`
      (set `self.Right` (select `int` 0 :`0` (struct :`Pitch` -20.0) :`1` (struct) :!type "Rotator Structure"))
      (`SceneComponent.K2_SetRelativeRotation` (`self.PlatformMesh`) (`self.StartRotation`) false false))))