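; Moveable platform that travels toward an endpoint once something overlaps its PlayerTouch trigger.
; BeginPlay caches the world locations of the Platform and Endpoint components as start and end points.
; The overlap plays a timeline whose track lerps the platform between them without sweep.
; The overlap does not filter the other actor, and ending it neither stops nor reverses the motion.
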(event `self.ReceiveBeginPlay`
  (set `self.StartLocation` (`SceneComponent.K2_GetComponentLocation` (`self.Platform`)))
  (set `self.EndLocation` (`SceneComponent.K2_GetComponentLocation` (`self.Endpoint`))))

(event `self.PlayerTouch.OnComponentBeginOverlap`
  (params (OverlappedComponent :type "PrimitiveComponent Object Reference") (OtherActor :type "Actor Object Reference") (OtherComp :type "PrimitiveComponent Object Reference") (OtherBodyIndex :type Integer) (bFromSweep :type Boolean) (SweepResult :type "HitResult Structure (by ref)"))
  (bind (_direction _newtrack_0) (`Timeline|Timeline_0`)
    (:`Update`
      (`SceneComponent.K2_SetWorldLocation` (`self.Platform`) (`KismetMathLibrary.VLerp` (`self.StartLocation`) (`self.EndLocation`) _newtrack_0) false false))))

(event `self.PlayerTouch.OnComponentEndOverlap`
  (params (OverlappedComponent :type "PrimitiveComponent Object Reference") (OtherActor :type "Actor Object Reference") (OtherComp :type "PrimitiveComponent Object Reference") (OtherBodyIndex :type Integer)))

(fn `UserConstructionScript`)